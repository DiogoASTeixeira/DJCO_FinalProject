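; SubtitlesManager is an actor that shows narration subtitles on screen one line at a time.
; On BeginPlay it creates a SubtitlesBP widget, adds it to the viewport and blanks it.
; ShowLine forwards to ShowNextLine, which reads the current row of the supplied narration DataTable, displays its LineToShow and advances the index.
; The NewLine flag restarts from the first row, and ClearSubtitles empties the display.
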(event Custom|Clear%20Subtitles
  (Default|DisplayLine (Variables|Default|GetSubtitlesWidgetRef)))

(event Custom|ShowNextLine
  (params (NewLine :type Boolean) (NarrationLines :type Data%20Table%20Object%20Reference))
  (Variables|Default|SetCurrentNarrationLine NarrationLines)
  (if NewLine
    (Variables|Default|SetCurrentRow 0)
    (bind _outrownames (DataTable|GetDataTableRowNames (Variables|Default|GetCurrentNarrationLine)))
    (bind _returnvalue (Utilities|GetDataTableRow (Variables|Default|GetCurrentNarrationLine) (Utilities|Array|Get(acopy) _outrownames (Variables|Default|GetCurrentRow)))
      (:then
        (Default|DisplayLine (Variables|Default|GetSubtitlesWidgetRef) (Utilities|Struct|BreakSubtitlesStruct _returnvalue))
        (Variables|Default|SetCurrentRow (+ (Variables|Default|GetCurrentRow) 1))))
    (else
      (bind _outrownames_2 (DataTable|GetDataTableRowNames (Variables|Default|GetCurrentNarrationLine)))
      (bind _returnvalue_2 (Utilities|GetDataTableRow (Variables|Default|GetCurrentNarrationLine) (Utilities|Array|Get(acopy) _outrownames_2 (Variables|Default|GetCurrentRow)))
        (:then
          (Default|DisplayLine (Variables|Default|GetSubtitlesWidgetRef) (Utilities|Struct|BreakSubtitlesStruct _returnvalue_2))
          (Variables|Default|SetCurrentRow (+ (Variables|Default|GetCurrentRow) 1)))))))

(event EventBeginPlay
  (bind _returnvalue (UserInterface|CreateWidget "/Game/Blueprint/SubtitlesBP.SubtitlesBP_C"))
  (bind _output_get (Variables|Default|SetSubtitlesWidgetRef _returnvalue))
  (UserInterface|Viewport|AddtoViewport _output_get 0)
  (CallFunction|ClearSubtitles))

(fn ConstructionScript)

(fn ShowLine
  (params (NewLine :type Boolean) (NarrationLines :type Data%20Table%20Object%20Reference))
  (CallFunction|ShowNextLine NewLine NarrationLines))