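; Game mode, apparently for the Motor level, that runs a countdown and opens the "Motor" level when time runs out.
; BeginPlay adds a Timer widget to the viewport.
; Tick uses a one-second Delay as a throttle to decrement Seconds, rolling over into Minutes, until both reach zero.
; A separate UpdateTimer function accumulates world delta seconds into StopTimer and returns it.
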(event EventBeginPlay
  (bind _returnvalue (UserInterface|CreateWidget "/Game/Blueprint/Timer.Timer_C"))
  (UserInterface|Viewport|AddtoViewport _returnvalue 0))

(event EventTick
  (params (DeltaSeconds :type Float%20%28single-precision%29))
  (Utilities|FlowControl|Delay 1.0)
  (Variables|Default|SetSeconds (- (Variables|Default|GetSeconds) 1))
  (if (< (Variables|Default|GetSeconds) 0)
    (Variables|Default|SetMinutes (- (Variables|Default|GetMinutes) 1))
    (Variables|Default|SetSeconds 59))
  (if (== (Variables|Default|GetSeconds) 0)
    (if (== (Variables|Default|GetMinutes) 0)
      (Game|OpenLevel(byName) "Motor"))))

(fn ConstructionScript)

(fn UpdateTimer
  (bind _output_get (Variables|Default|SetStop%20Timer (+ (Variables|Default|GetStop%20Timer) (Utilities|Time|GetWorldDeltaSeconds))))
  (return _output_get))